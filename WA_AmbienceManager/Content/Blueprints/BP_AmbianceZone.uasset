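; BP_AmbianceZone is a trigger volume that tells the player character which ambiance zone it has entered, covering Kioki and Saborian deserts and forests.
; When an actor of the player character's class begins overlapping the Box, it calls NewZoneMessage on that actor with the zone's ZoneType.
; The construction script sets the TextRender label to the name of the selected ZoneType.
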(event `self.Box.OnComponentBeginOverlap`
  (params (OverlappedComponent :type "PrimitiveComponent Object Reference") (OtherActor :type "Actor Object Reference") (OtherComp :type "PrimitiveComponent Object Reference") (OtherBodyIndex :type Integer) (bFromSweep :type Boolean) (SweepResult :type "HitResult Structure (by ref)"))
  (if (== (`GameplayStatics.GetObjectClass` OtherActor) (`GameplayStatics.GetObjectClass` (`GameplayStatics.GetPlayerCharacter` 0)))
    (message `/WA_AmbienceManager/Blueprints/BPI_PlayerChangeZone.NewZone` OtherActor (`self.ZoneType`))))

(fn `UserConstructionScript`
  (`TextRenderComponent.K2_SetText` (`self.TextRender`) (select `/WA_AmbienceManager/Blueprints/ENUM_ZoneType` (`self.ZoneType`) :`NewEnumerator0` "Kioki Desert" :`NewEnumerator1` "Saborian Desert" :`NewEnumerator2` "Kioki Forest" :`NewEnumerator3` "Saborian Forest")))