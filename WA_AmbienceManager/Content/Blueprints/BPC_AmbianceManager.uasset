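; Actor component that manages looping 2D zone ambience as the game moves between the Kioki and Saborian desert and forest zones.
; A NewZone event stores the latest zone, fades out and stops the current ambience, then spawns that zone's daytime sound cue at reduced volume.
; Short delays separate the fade from the spawn, and the cue is chosen from the stored zone once they finish.
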(event `self.ReceiveBeginPlay`)

(event `/WA_AmbienceManager/Blueprints/BPI_PlayerChangeZone.NewZone`
  (params (Zone_Type :type "/WA_AmbienceManager/Blueprints/ENUM_ZoneType Enum" :default "NewEnumerator0"))
  (bind _ambiance_soundcue (`self.Ambiance_SoundCUE`))
  (set `self.LatestZone` Zone_Type)
  (`/Engine/EditorBlueprintResources/StandardMacros.IsValid` _ambiance_soundcue
    (:`Is Valid`
      (`AudioComponent.FadeOut` _ambiance_soundcue 1.5 0.0 "Linear")
      (`KismetSystemLibrary.Delay` 2.0)
      (`/Engine/EditorBlueprintResources/StandardMacros.IsValid` _ambiance_soundcue
        (:`Is Valid`
          (`AudioComponent.Stop` _ambiance_soundcue))
        (:`Is Not Valid`
          _))
      (set `self.Ambiance_SoundCUE` null))
    (:`Is Not Valid`
      _))
  (`KismetSystemLibrary.Delay` 0.05)
  (bind _returnvalue (`GameplayStatics.SpawnSound2D` (select `/WA_AmbienceManager/Blueprints/ENUM_ZoneType` (`self.LatestZone`) :`NewEnumerator0` "/WA_AmbienceManager/Musics/CUEs/CUE_Kioki_Desert_Day.CUE_Kioki_Desert_Day" :`NewEnumerator1` "/WA_AmbienceManager/Musics/CUEs/CUE_Saborian_Desert_Day.CUE_Saborian_Desert_Day" :`NewEnumerator2` "/WA_AmbienceManager/Musics/CUEs/CUE_Kioki_Forest_Day.CUE_Kioki_Forest_Day" :`NewEnumerator3` "/WA_AmbienceManager/Musics/CUEs/CUE_Saborian_Forest_Day.CUE_Saborian_Forest_Day" :!type "SoundBase Object Reference") 0.5 1.0 0.0 null))
  (set `self.Ambiance_SoundCUE` _returnvalue))